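; Test actor that benchmarks sorting algorithms on random float, string, integer and byte arrays.
; Events generate arrays, dispatch by algorithm enum to function or macro sorts, then print elapsed time and optionally the elements, which inflates timings.
; Timing uses only clock seconds and milliseconds, so it breaks across minute rollovers; the macro event's Integer and Float cases are swapped.
; Another event shuffles all level actors, sorts them, reverses and prints their names.
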(event Custom|TestSortActors
  (bind _outactors (Actor|GetAllActorsOfClass "/Script/Engine.Actor"))
  (Utilities|Array|Shuffle _outactors)
  (CallFunction|SortActors _outactors "NewEnumerator3")
  (Utilities|Array|Reverse _outactors)
  (for _array_element _outactors
    (Development|PrintString (Utilities|GetDisplayName _array_element) true true "(R=0.000000,G=0.660000,B=1.000000,A=1.000000)" 22.0)))

(event Custom|SortWithMacroEvent
  (bind _macrotestsize (Variables|Default|Macro|GetMacroTestSize))
  (bind _macrosortalgorithm (Variables|Default|Macro|GetMacroSortAlgorithm))
  (bind _log_array (Variables|Default|GetLog%20Array))
  ;[0 0 0] MACRO
  (switch Utilities|FlowControl|Switch|SwitchonE_SortingDataType (Variables|Default|Macro|GetMacroDataType)
    (:NewEnumerator0
      (Testing|Macro|DebugFloatsSortingMacro _macrosortalgorithm _macrotestsize _log_array))
    (:NewEnumerator1
      (Testing|Macro|DebugIntsSortingMacro _macrosortalgorithm _macrotestsize _log_array))
    (:NewEnumerator2
      (Testing|Macro|DebugBytesSortingMacro _macrosortalgorithm _macrotestsize _log_array))))

(event Custom|SortStringsEvent
  ;[0 0 0] Functions
  (Testing|DebugStringsSorting (Variables|Default|Strings|GetStringSortingAlgorithm) (Variables|Default|Strings|GetStringArraySize) (Variables|Default|GetLog%20Array)))

(event Custom|SortFloatsEvent
  ;[0 0 0] Functions
  (Testing|DebugFloatsSorting (Variables|Default|Floats|GetFloatSortingAlgorithm) (Variables|Default|Floats|GetFloatArraySize) (Variables|Default|GetLog%20Array)))

(fn ConstructionScript)

(fn MakeIntArray
  (params (LastIndex :type Integer))
  (for _index (range 0 LastIndex)
    (Utilities|Array|Add (LocalVariables|GetLocalArray) (Math|Random|RandomIntegerinRange 0 LastIndex)))
  (return (LocalVariables|GetLocalArray)))

(fn MakeFloatArray
  (params (LastIndex :type Integer))
  (for _index (range 0 LastIndex)
    (if (> (Math|Random|RandomIntegerinRange 0 9) 0)
      (Utilities|Array|Add (LocalVariables|GetLocalArray) (Math|Random|RandomFloatinRange 0.0 (Math|Conversions|ToFloat(Integer) LastIndex)))
      (else
        (Utilities|Array|Add (LocalVariables|GetLocalArray) (.OutItem (Utilities|Array|Random (LocalVariables|GetLocalArray)))))))
  (return (LocalVariables|GetLocalArray)))

(fn MakeStringArray
  (params (LastIndex :type Integer))
  (for _index (range 0 LastIndex)
    (if (> (Math|Random|RandomIntegerinRange 0 9) 0)
      (Utilities|Array|Add (LocalVariables|GetLocalArray) (Testing|MakeArray|MakeRandomString))
      (else
        (Utilities|Array|Add (LocalVariables|GetLocalArray) (.OutItem (Utilities|Array|Random (LocalVariables|GetLocalArray)))))))
  (return (LocalVariables|GetLocalArray)))

(fn SecondsStamp
  (bind _returnvalue (Math|DateTime|Now))
  (return (+ (Math|Conversions|ToFloat(Integer) (.second _returnvalue)) (/ (Math|Conversions|ToFloat(Integer) (.millisecond _returnvalue)) 1e+03))))

(fn SortwithAlgorithm
  (params (Array :type Array%20of%20Floats%20%28double-precision%29) (Algorithm :type E_SortingAlgorithms%20Enum :default "NewEnumerator0"))
  (switch Utilities|FlowControl|Switch|SwitchonE_SortingAlgorithms Algorithm
    (:NewEnumerator0
      (CallFunction|BubbleSortFloat Array))
    (:NewEnumerator1
      (CallFunction|SelSortFloat Array))
    (:NewEnumerator2
      (CallFunction|InsertSortFloat Array))
    (:NewEnumerator3
      (CallFunction|CombSortFloat Array))
    (:NewEnumerator6
      (CallFunction|ShellSortFloat Array))
    (:NewEnumerator4
      (CallFunction|QuickSortFloat Array))
    (:NewEnumerator5
      (CallFunction|IntroSortFloat Array))
    (:NewEnumerator7
      (CallFunction|WildSelSortFloat Array))))

(fn SortStringwithAlgorithm
  (params (Array :type Array%20of%20Strings) (Algorithm :type E_SortingAlgorithms%20Enum :default "NewEnumerator0"))
  (switch Utilities|FlowControl|Switch|SwitchonE_SortingAlgorithms Algorithm
    (:NewEnumerator0
      (CallFunction|BubbleSortString Array))
    (:NewEnumerator3
      (CallFunction|CombSortString Array))
    (:NewEnumerator4
      (CallFunction|QuickSortString Array))
    (:NewEnumerator5
      (CallFunction|IntroSortString Array))))

(fn DebugFloatsSorting
  (params (Method :type E_SortingAlgorithms%20Enum :default "NewEnumerator0") (LastIndex :type Integer) (LogArray :type Boolean))
  (bind _array (Testing|MakeArray|MakeFloatArray LastIndex))
  (Development|PrintString (Utilities|String|Append "START  " (Utilities|String|EnumtoString Method)))
  (bind _returnvalue (Testing|Time|SecondsStamp))
  (Testing|SortwithAlgorithm _array Method)
  (Utilities|FlowControl|Sequence
    (:then_0
      (if LogArray
        (for _array_element _array
          (Development|PrintString (Utilities|String|ToString(Float) _array_element) false))))
    (:then_1
      (bind _returnvalue_2 (Testing|Time|SecondsStamp))
      (Development|PrintString (Utilities|String|Append "END  " (Utilities|String|EnumtoString Method) "  --  " (Utilities|String|ToString(Float) (- _returnvalue_2 _returnvalue)))))))

(fn DebugStringsSorting
  (params (Method :type E_SortingAlgorithms%20Enum :default "NewEnumerator0") (LastIndex :type Integer) (LogArray :type Boolean))
  (bind _array (Testing|MakeArray|MakeStringArray LastIndex))
  (Development|PrintString (Utilities|String|Append "START  " (Utilities|String|EnumtoString Method)))
  (bind _returnvalue (Testing|Time|SecondsStamp))
  (Testing|SortStringwithAlgorithm _array Method)
  (Utilities|FlowControl|Sequence
    (:then_0
      (if LogArray
        (for _array_element _array
          (Development|PrintString _array_element false))))
    (:then_1
      (bind _returnvalue_2 (Testing|Time|SecondsStamp))
      (Development|PrintString (Utilities|String|Append "END  " (Utilities|String|EnumtoString Method) "  --  " (Utilities|String|ToString(Float) (- _returnvalue_2 _returnvalue)))))))

(fn MakeByteArray
  (params (LastIndex :type Integer))
  (for _index (range 0 LastIndex)
    (Utilities|Array|Add (LocalVariables|GetLocalArray) (Math|Conversions|ToByte(Integer) (Math|Random|RandomIntegerinRange 0 255))))
  (return (LocalVariables|GetLocalArray)))

(fn DebugMacroSorting
  (params (Method :type E_SortingAlgorithms%20Enum :default "NewEnumerator0") (LastIndex :type Integer) (Print :type Boolean))
  (bind _array (Testing|MakeArray|MakeFloatArray LastIndex))
  (Development|PrintString (Utilities|String|Append "START  " (Utilities|String|EnumtoString Method)))
  (bind _returnvalue (Testing|Time|SecondsStamp))
  (Testing|Macro|SortFloatswithMacro _array Method)
  (Utilities|FlowControl|Sequence
    (:then_0
      (if Print
        (for _array_element _array
          (Development|PrintString (Utilities|String|ToString(Float) _array_element)))))
    (:then_1
      (bind _returnvalue_2 (Testing|Time|SecondsStamp))
      (Development|PrintString (Utilities|String|Append "END  " (Utilities|String|EnumtoString Method) "  --  " (Utilities|String|ToString(Float) (- _returnvalue_2 _returnvalue)))))))

(fn SortFloatswithMacro
  (params (Array :type Array%20of%20Floats%20%28double-precision%29) (Algorithm :type E_SortingAlgorithms%20Enum :default "NewEnumerator0"))
  (switch Utilities|FlowControl|Switch|SwitchonE_SortingAlgorithms Algorithm
    (:NewEnumerator0
      (Utilities|BubbleSortMacro Array))
    (:NewEnumerator1
      (Utilities|SelectionSortMacro Array))
    (:NewEnumerator2
      (Utilities|InsertionSortMacro Array))
    (:NewEnumerator3
      (Utilities|CombSortMacro Array))
    (:NewEnumerator6
      (Utilities|ShellSortMacro Array))))

(fn SwitchFuncMacroFloats
  (params (Macro :type Boolean) (Array :type Array%20of%20Floats%20%28double-precision%29) (Algorithm :type E_SortingAlgorithms%20Enum :default "NewEnumerator0"))
  (if Macro
    (Testing|SortwithAlgorithm Array "NewEnumerator0")
    (else
      (Testing|Macro|SortFloatswithMacro Array Algorithm))))

(fn SortIntswithMacro
  (params (Array :type Array%20of%20Integers) (Algorithm :type E_SortingAlgorithms%20Enum :default "NewEnumerator0"))
  (switch Utilities|FlowControl|Switch|SwitchonE_SortingAlgorithms Algorithm
    (:NewEnumerator0
      (Utilities|BubbleSortMacro Array))
    (:NewEnumerator1
      (Utilities|SelectionSortMacro Array))
    (:NewEnumerator2
      (Utilities|InsertionSortMacro Array))
    (:NewEnumerator3
      (Utilities|CombSortMacro Array))
    (:NewEnumerator6
      (Utilities|ShellSortMacro Array))))

(fn DebugFloatsSortingMacro
  (params (Method :type E_SortingAlgorithms%20Enum :default "NewEnumerator0") (LastIndex :type Integer) (LogArray :type Boolean))
  (bind _array (Testing|MakeArray|MakeFloatArray LastIndex))
  (Development|PrintString (Utilities|String|Append "START MACRO floats  " (Utilities|String|EnumtoString Method)))
  (bind _returnvalue (Testing|Time|SecondsStamp))
  (Testing|Macro|SortFloatswithMacro _array Method)
  (Utilities|FlowControl|Sequence
    (:then_0
      (if LogArray
        (for _array_element _array
          (Development|PrintString (Utilities|String|ToString(Float) _array_element) false))))
    (:then_1
      (bind _returnvalue_2 (Testing|Time|SecondsStamp))
      (Development|PrintString (Utilities|String|Append "END  " (Utilities|String|EnumtoString Method) "  --  " (Utilities|String|ToString(Float) (- _returnvalue_2 _returnvalue)))))))

(fn DebugIntsSortingMacro
  (params (Method :type E_SortingAlgorithms%20Enum :default "NewEnumerator0") (LastIndex :type Integer) (LogArray :type Boolean))
  (bind _array (Testing|MakeArray|MakeIntArray LastIndex))
  (Development|PrintString (Utilities|String|Append "START  MACRO Integers" (Utilities|String|EnumtoString Method)))
  (bind _returnvalue (Testing|Time|SecondsStamp))
  (Testing|Macro|SortIntswithMacro _array Method)
  (Utilities|FlowControl|Sequence
    (:then_0
      (if LogArray
        (for _array_element _array
          (Development|PrintString (Utilities|String|ToString(Integer) _array_element) false))))
    (:then_1
      (bind _returnvalue_2 (Testing|Time|SecondsStamp))
      (Development|PrintString (Utilities|String|Append "END  " (Utilities|String|EnumtoString Method) "  --  " (Utilities|String|ToString(Float) (- _returnvalue_2 _returnvalue)))))))

(fn DebugBytesSortingMacro
  (params (Method :type E_SortingAlgorithms%20Enum :default "NewEnumerator0") (LastIndex :type Integer) (LogArray :type Boolean))
  (bind _array (Testing|MakeArray|MakeByteArray LastIndex))
  (Development|PrintString (Utilities|String|Append "START  MACRO Bytes" (Utilities|String|EnumtoString Method)))
  (bind _returnvalue (Testing|Time|SecondsStamp))
  (Testing|Macro|SortByteswithMacro _array Method)
  (Utilities|FlowControl|Sequence
    (:then_0
      (if LogArray
        (for _array_element _array
          (Development|PrintString (Utilities|String|ToString(Byte) _array_element) false))))
    (:then_1
      (bind _returnvalue_2 (Testing|Time|SecondsStamp))
      (Development|PrintString (Utilities|String|Append "END  " (Utilities|String|EnumtoString Method) "  --  " (Utilities|String|ToString(Float) (- _returnvalue_2 _returnvalue)))))))

(fn SortByteswithMacro
  (params (Array :type Array%20of%20Bytes) (Algorithm :type E_SortingAlgorithms%20Enum :default "NewEnumerator0"))
  (switch Utilities|FlowControl|Switch|SwitchonE_SortingAlgorithms Algorithm
    (:NewEnumerator0
      (Utilities|BubbleSortMacro Array))
    (:NewEnumerator1
      (Utilities|SelectionSortMacro Array))
    (:NewEnumerator2
      (Utilities|InsertionSortMacro Array))
    (:NewEnumerator3
      (Utilities|CombSortMacro Array))
    (:NewEnumerator6
      (Utilities|ShellSortMacro Array))))

(fn MakeRandomString
  (bind _output_get (LocalVariables|SetTempChars (Utilities|String|GetCharacterArrayfromString (LocalVariables|GetChars))))
  (Utilities|Array|Shuffle _output_get)
  (return (Utilities|String|GetSubstring (Utilities|String|JoinStringArray _output_get "") (Math|Random|RandomIntegerinRange 0 (- (Utilities|String|Len (LocalVariables|GetChars)) 10)) (Math|Random|RandomIntegerinRange 5 12))))